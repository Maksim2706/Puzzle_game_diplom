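; BP_LVL_WIN is a level-finish trigger that records the player's completion and returns to FirstPersonMap.
; On BeginPlay it loads the save and flags which LvLNames entry matches the current level.
; Box overlap by the player enables input and opens a gate for the Interract action.
; Interacting writes that level's completion, HUD time and a minutes-based score to the save, then opens the map after a short delay.
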(event OnComponentBeginOverlap(Box)
  (params (OverlappedComponent :type Primitive%20Component%20Object%20Reference) (OtherActor :type Actor%20Object%20Reference) (OtherComp :type Primitive%20Component%20Object%20Reference) (OtherBodyIndex :type Integer) (bFromSweep :type Boolean) (SweepResult :type Hit%20Result%20Structure%20%28by%20ref%29))
  (bind _as_bp_game_save (Variables|Default|GetAs%20BP%20Game%20Save))
  (Utilities|Casting|CastToBP_FirstPersonCharacter OtherActor)
  (Input|EnableInput (Game|GetPlayerController 0))
  (Utilities|FlowControl|Gate true) ; enters at Open
)

(event OnComponentEndOverlap(Box)
  (params (OverlappedComponent :type Primitive%20Component%20Object%20Reference) (OtherActor :type Actor%20Object%20Reference) (OtherComp :type Primitive%20Component%20Object%20Reference) (OtherBodyIndex :type Integer))
  (bind _as_bp_game_save (Variables|Default|GetAs%20BP%20Game%20Save))
  (Utilities|Casting|CastToBP_FirstPersonCharacter OtherActor)
  (Input|DisableInput (Game|GetPlayerController 0))
  (Utilities|FlowControl|Gate true) ; enters at Close
)

(event EventBeginPlay
  ;[1 1 1] LvL check
  (bind _returnvalue (SaveGame|LoadGamefromSlot "Save1"))
  (bind _asbp_game_save (Utilities|Casting|CastToBP_GameSave _returnvalue))
  (Variables|Default|SetAs%20BP%20Game%20Save _asbp_game_save)
  (bind _returnvalue_2 (Game|GetCurrentLevelName true))
  (for (_array_element _array_index) (Variables|Default|GetLvL%20names)
    (Utilities|Array|SetArrayElem (Variables|Default|GetIsLvL) _array_index (== _array_element (Utilities|String|StringToName _returnvalue_2)))))

(event Input|ActionEvents|InputActionInterract
  (params (Key :type Key%20Structure :default "None"))
  (bind _as_bp_game_save (Variables|Default|GetAs%20BP%20Game%20Save))
  (:Pressed
    (Utilities|FlowControl|Gate true
      (:Exit
        (bind _ashud_bp (Utilities|Casting|CastToHUD_BP (HUD|GetHUD (Game|GetPlayerController 0))))
        (for (_array_element _array_index) (Variables|Default|GetIsLvL)
          (if _array_element
            (Utilities|Array|SetArrayElem (Variables|/Game/FP_Maps/Save_game/BP_GameSave.BP_GameSave_C|GetCompleted_LVL _as_bp_game_save) _array_index true)
            (if _array_element
              (Utilities|Array|SetArrayElem (Variables|/Game/FP_Maps/Save_game/BP_GameSave.BP_GameSave_C|GetLvL_Time_Min _as_bp_game_save) _array_index (Variables|/Game/FirstPerson/Blueprints/HUD_BP.HUD_BP_C|GetTimeMin _ashud_bp))
              (Utilities|Array|SetArrayElem (Variables|/Game/FP_Maps/Save_game/BP_GameSave.BP_GameSave_C|GetLvL_Time_Sec _as_bp_game_save) _array_index (Variables|/Game/FirstPerson/Blueprints/HUD_BP.HUD_BP_C|GetTimeSec _ashud_bp))
              (Utilities|Array|SetArrayElem (Variables|/Game/FP_Maps/Save_game/BP_GameSave.BP_GameSave_C|GetLvL_Score _as_bp_game_save) _array_index (/ 1000 (+ (Variables|/Game/FirstPerson/Blueprints/HUD_BP.HUD_BP_C|GetTimeMin _ashud_bp) 1))))))
        (SaveGame|SaveGametoSlot (Variables|Default|GetAs%20BP%20Game%20Save) "Save1")
        (Utilities|FlowControl|Delay 0.2)
        (Game|OpenLevel(byObjectReference) "/Game/FP_Maps/FirstPersonMap.FirstPersonMap")))))

(fn ConstructionScript)